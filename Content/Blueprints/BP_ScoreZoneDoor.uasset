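; BP_ScoreZoneDoor is a trigger actor that locks doors once the first-person player character leaves its Box volume.
; The first matching end overlap passes a DoOnce, then loops over the child actors of the Door component's child actor.
; Each one that casts to BP_DoorInteractable prints a debug "Success" and has LockDoors called on it.
; Despite the name, it contains no scoring logic.
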(event `self.Box.OnComponentEndOverlap`
  (params (OverlappedComponent :type "PrimitiveComponent Object Reference") (OtherActor :type "Actor Object Reference") (OtherComp :type "PrimitiveComponent Object Reference") (OtherBodyIndex :type Integer))
  (cast `/Game/FirstPerson/Blueprints/BP_FirstPersonCharacter` OtherActor)
  (`/Engine/EditorBlueprintResources/StandardMacros.DoOnce` false
    (:`Completed`
      (for _array_element (`self.GetAllChildActors` (`ChildActorComponent.ChildActor` (`self.Door`)) true)
        (bind _asbp_door_interactable (cast `/Game/Blueprints/Kitbash/Tiles/BP_DoorInteractable` _array_element))
        (`KismetSystemLibrary.PrintString` "Success")
        (`/Game/Blueprints/Kitbash/Tiles/BP_DoorInteractable.LockDoors` _asbp_door_interactable)))))

(fn `UserConstructionScript`
  (`parent.UserConstructionScript`))