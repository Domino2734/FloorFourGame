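; Interactable door tile that swings on a timeline, with open and close sounds, and gets a random hue on its dynamic material.
; Triggering alternates opening and closing through a FlipFlop, or only plays a sound when locked.
; A timeline event track times the close sound during reverse playback.
; LockDoors locks and shuts an open door, while UnlockDoors unlocks and toggles only puzzle-room exits.
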(event `self.ReceiveBeginPlay`
  (`parent.ReceiveBeginPlay`)
  (`self.RandomColour` (`self.StaticMesh`)))

(event `ToggleDoor`
  ;[0.15 0 0 0.5] Door Slam (anim+audio)
  (bind _isa (`/Engine/EditorBlueprintResources/StandardMacros.FlipFlop` :!label _label)
    (:`A`
      (`AudioComponent.Play` (`self.Audio`) 0.0)
      (bind (_direction _rotation) (`Timeline|OpenDoor` :!label _label_2)
        (:`Update`
          (`SceneComponent.K2_SetRelativeRotation` (`self.StaticMesh`) (`KismetMathLibrary.MakeRotator` 90.0 0.0 _rotation) false false)
          (set `self.isOpen` true))
        (:`DoorCloseAudioTrigger`
          (if (not _isa)
            (`AudioComponent.Play` (`self.Audio1`) 0.0)
            (set `self.isOpen` false)))))
    (:`B`
      (goto _label_2 :!via `ReverseFromEnd`))))

(event `self.Triggered`
  (if (`self.isLocked`)
    (`AudioComponent.Play` (`self.Audio`) 0.5)
    (`KismetSystemLibrary.Delay` 0.25)
    (else
      (goto _label))))

(event `LockDoors`
  (set `self.isLocked` true)
  (if (`self.isOpen`)
    (goto _label)))

(event `UnlockDoors`
  (if (`self.isPuzzleRoomExit`)
    (set `self.isLocked` false)
    (goto _label)))

(fn `RandomColour`
  (params (Target :type "PrimitiveComponent Object Reference"))
  (bind _returnvalue (`KismetMaterialLibrary.CreateDynamicMaterialInstance` "/Game/Models/KitbashTiles/Walls/Textures/M_Door.M_Door" "None" "Transient"))
  (`PrimitiveComponent.SetMaterial` Target 0 _returnvalue)
  (`MaterialInstanceDynamic.SetScalarParameterValue` _returnvalue "Hue" (`KismetMathLibrary.RandomFloatInRange` 0.6 1.2)))

(fn `UserConstructionScript`
  (`parent.UserConstructionScript`)
  (`self.RandomColour` (`self.StaticMesh`)))