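; Kitbash hallway segment, apparently with a light, that gives its two door meshes varied colouring.
; The construction script creates a separate dynamic instance of M_Door for each door and sets its Hue parameter to an independent random value within a limited range.
; Random-colour vector nodes are left disconnected, and the event graph holds only disabled default events.
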(fn `UserConstructionScript`
  (bind _returnvalue (`KismetMaterialLibrary.CreateDynamicMaterialInstance` "/Game/Models/KitbashTiles/Walls/Textures/M_Door.M_Door" "None" "Transient"))
  (`PrimitiveComponent.SetMaterial` (`self.Door`) 0 _returnvalue)
  (`MaterialInstanceDynamic.SetScalarParameterValue` _returnvalue "Hue" (`KismetMathLibrary.RandomFloatInRange` 0.6 1.2))
  (bind _returnvalue_2 (`KismetMaterialLibrary.CreateDynamicMaterialInstance` "/Game/Models/KitbashTiles/Walls/Textures/M_Door.M_Door" "None" "Transient"))
  (`PrimitiveComponent.SetMaterial` (`self.Door1`) 0 _returnvalue_2)
  (`MaterialInstanceDynamic.SetScalarParameterValue` _returnvalue_2 "Hue" (`KismetMathLibrary.RandomFloatInRange` 0.6 1.2)))