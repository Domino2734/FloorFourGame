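; BP_Interactable is an interactable object with a static mesh that carries a good or bad score value.
; On BeginPlay, UpdateScoreValue converts the Score category into signed Points, scaled across three magnitudes each way.
; The construction script disallows Nanite on the mesh.
; The Triggered event is empty, and leftover unconnected nodes set IsActivated, print debug text and decrement SpawnsLeft on a parent BP_InfiniteHallway.
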(event `self.ReceiveBeginPlay`
  (`self.UpdateScoreValue`))

(event `Triggered`)

(fn `UpdateScoreValue`
  (switch `/Game/Blueprints/Enums/EN_ScoreValues` (`self.Score`)
    (:`NewEnumerator0`
      (set `self.Points` -30.0))
    (:`NewEnumerator1`
      (set `self.Points` -15.0))
    (:`NewEnumerator4`
      (set `self.Points` -7.0))
    (:`NewEnumerator5`
      (set `self.Points` 7.0))
    (:`NewEnumerator2`
      (set `self.Points` 15.0))
    (:`NewEnumerator3`
      (set `self.Points` 30.0)))
  (return))

(fn `UserConstructionScript`
  (set `StaticMeshComponent.bDisallowNanite` true (`self.StaticMesh`)))