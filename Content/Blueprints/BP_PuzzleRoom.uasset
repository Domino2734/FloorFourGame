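; BP_PuzzleRoom is a timed story room that temporarily locks the player in.
; On BeginPlay it toggles every BP_DoorInteractable overlapping StoryRoomArea.
; The first StoryRoomTrigger overlap locks those doors if the actor is BP_FirstPersonCharacter, and regardless starts an OpenAfterSecs delay before calling OpenExit.
; OpenExit unlocks the area's doors, with DoOnce gates keeping both trigger and exit single-use.
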(event `self.ReceiveBeginPlay`
  (for _array_element (`PrimitiveComponent.GetOverlappingActors` (`self.StoryRoomArea`) "/Game/Blueprints/Kitbash/Tiles/BP_DoorInteractable.BP_DoorInteractable_C")
    (bind _asbp_door_interactable (cast `/Game/Blueprints/Kitbash/Tiles/BP_DoorInteractable` _array_element))
    (`/Game/Blueprints/Kitbash/Tiles/BP_DoorInteractable.ToggleDoor` _asbp_door_interactable)))

(event `self.StoryRoomTrigger.OnComponentBeginOverlap`
  (params (OverlappedComponent :type "PrimitiveComponent Object Reference") (OtherActor :type "Actor Object Reference") (OtherComp :type "PrimitiveComponent Object Reference") (OtherBodyIndex :type Integer) (bFromSweep :type Boolean) (SweepResult :type "HitResult Structure (by ref)"))
  (`/Engine/EditorBlueprintResources/StandardMacros.DoOnce` false
    (:`Completed`
      (`|ExecutionSequence`
        (:`then_0`
          (cast `/Game/FirstPerson/Blueprints/BP_FirstPersonCharacter` OtherActor)
          (for _array_element (`PrimitiveComponent.GetOverlappingActors` (`self.StoryRoomArea`) "/Game/Blueprints/Kitbash/Tiles/BP_DoorInteractable.BP_DoorInteractable_C")
            (bind _asbp_door_interactable (cast `/Game/Blueprints/Kitbash/Tiles/BP_DoorInteractable` _array_element))
            (`/Game/Blueprints/Kitbash/Tiles/BP_DoorInteractable.LockDoors` _asbp_door_interactable)))
        (:`then_1`
          (`KismetSystemLibrary.Delay` (`self.OpenAfterSecs`))
          (`self.OpenExit`))))))

(event `OpenExit`
  (`/Engine/EditorBlueprintResources/StandardMacros.DoOnce` false
    (:`Completed`
      (for _array_element (`PrimitiveComponent.GetOverlappingActors` (`self.StoryRoomArea`) "/Game/Blueprints/Kitbash/Tiles/BP_DoorInteractable.BP_DoorInteractable_C")
        (bind _asbp_door_interactable (cast `/Game/Blueprints/Kitbash/Tiles/BP_DoorInteractable` _array_element))
        (`/Game/Blueprints/Kitbash/Tiles/BP_DoorInteractable.UnlockDoors` _asbp_door_interactable)))))

(fn `UserConstructionScript`)