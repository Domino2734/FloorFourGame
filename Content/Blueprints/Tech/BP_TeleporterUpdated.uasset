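; Teleporter actor that moves a Character entering TeleportStartZone to TeleportEndMarker, carrying over its offset from TeleportStartMarker.
; The first overlapping Character is cached, and later overlaps teleport only that one.
; The offset is rotated about Z by the unsigned angle between marker forward vectors, and control yaw shifts by the markers' yaw difference.
; Velocity is multiplied component-wise by the end marker's normalized rotation angles rather than rotated.
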(event `self.TeleportStartZone.OnComponentBeginOverlap`
  (params (OverlappedComponent :type "PrimitiveComponent Object Reference") (OtherActor :type "Actor Object Reference") (OtherComp :type "PrimitiveComponent Object Reference") (OtherBodyIndex :type Integer) (bFromSweep :type Boolean) (SweepResult :type "HitResult Structure (by ref)"))
  (bind _as_character (`self.As Character`))
  (bind (_returnvalue_roll _returnvalue_pitch _returnvalue_yaw) (`KismetMathLibrary.BreakRotator` (`SceneComponent.K2_GetComponentRotation` (`self.TeleportStartMarker`))))
  (bind (_returnvalue_roll_2 _returnvalue_pitch_2 _returnvalue_yaw_2) (`KismetMathLibrary.BreakRotator` (`Pawn.GetControlRotation` _as_character)))
  (bind (_returnvalue_roll_3 _returnvalue_pitch_3 _returnvalue_yaw_3) (`KismetMathLibrary.BreakRotator` (`SceneComponent.K2_GetComponentRotation` (`self.TeleportEndMarker`))))
  ;[0.15 0 0 0.5] Skip player cast if already cached
  (`/Engine/EditorBlueprintResources/StandardMacros.IsValid` (`self.As Character`)
    (:`Is Valid`
      (if (== OtherActor (`self.As Character`))
        ; Change Location
        (`self.K2_SetActorLocation` (`self.As Character`) (+ (`KismetMathLibrary.RotateAngleAxis` (- (`self.K2_GetActorLocation` (`self.As Character`)) (`SceneComponent.K2_GetComponentLocation` (`self.TeleportStartMarker`))) (`KismetMathLibrary.DegAcos` (`KismetMathLibrary.Dot_VectorVector` (`SceneComponent.GetForwardVector` (`self.TeleportStartMarker`)) (`SceneComponent.GetForwardVector` (`self.TeleportEndMarker`)))) (0.0 0.0 1.0)) (`SceneComponent.K2_GetComponentLocation` (`self.TeleportEndMarker`))) false false :!label _label)
        ; Fix the velocity when rotating
        (set `MovementComponent.Velocity` (* (`self.GetVelocity` _as_character) (`KismetMathLibrary.Normal` (`KismetMathLibrary.MakeVector` _returnvalue_roll_3 _returnvalue_pitch_3 _returnvalue_yaw_3))) (`Character.CharacterMovement` _as_character))
        ; Change Rotation
        (`Controller.SetControlRotation` (`Pawn.GetController` _as_character) (`KismetMathLibrary.MakeRotator` _returnvalue_roll_2 _returnvalue_pitch_2 (+ (- _returnvalue_yaw_2 _returnvalue_yaw) _returnvalue_yaw_3)))))
    (:`Is Not Valid`
      ;[1 0.25 0 0.5] Replace Cast to Character with Cast to [PLAYER]
      (bind _ascharacter (cast `Character` OtherActor))
      (`KismetSystemLibrary.PrintString` (`KismetSystemLibrary.GetDisplayName` _ascharacter))
      (set `self.As Character` _ascharacter)
      (goto _label))))

(fn `UserConstructionScript`)