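; BP_EndTeleport is an ending selector that teleports the first-person player to one of three ending markers by Score.
; On overlapping the start zone, it caches the player character and picks the target marker from two score thresholds.
; It carries the player's offset from the start marker over to the target, rotated about Z by the angle between marker forwards.
; Control yaw shifts by the markers' yaw difference, and velocity is scaled by the target's normalized rotation.
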(event `self.TeleportStartZone.OnComponentBeginOverlap`
  (params (OverlappedComponent :type "PrimitiveComponent Object Reference") (OtherActor :type "Actor Object Reference") (OtherComp :type "PrimitiveComponent Object Reference") (OtherBodyIndex :type Integer) (bFromSweep :type Boolean) (SweepResult :type "HitResult Structure (by ref)"))
  (bind _as_character (`self.As Character`))
  (bind (_returnvalue_roll _returnvalue_pitch _returnvalue_yaw) (`KismetMathLibrary.BreakRotator` (`SceneComponent.K2_GetComponentRotation` (`self.TeleportStartMarker`))))
  (bind (_returnvalue_roll_2 _returnvalue_pitch_2 _returnvalue_yaw_2) (`KismetMathLibrary.BreakRotator` (`Pawn.GetControlRotation` _as_character)))
  (bind (_returnvalue_roll_3 _returnvalue_pitch_3 _returnvalue_yaw_3) (`KismetMathLibrary.BreakRotator` (`SceneComponent.K2_GetComponentRotation` (`self.TeleportTarget`))))
  ;[0.15 0 0 0.5] Skip player cast if already cached
  (`/Engine/EditorBlueprintResources/StandardMacros.IsValid` (`self.As Character`)
    (:`Is Valid`
      (if (== OtherActor (`self.As Character`))
        (bind _score (`/Game/FirstPerson/Blueprints/BP_FirstPersonCharacter.Score` (stale _asbp_first_person_character)))
        (if (>= _score 30.0) :!label _label
          (set `self.TeleportTarget` (`self.EndingOneMarker`))
          (elif (>= _score -30.0)
            (set `self.TeleportTarget` (`self.EndingTwoMarker`))
            (else
              (set `self.TeleportTarget` (`self.EndingThreeMarker`)))))
        ; Change Location
        (`self.K2_SetActorLocation` (`self.As Character`) (+ (`KismetMathLibrary.RotateAngleAxis` (- (`self.K2_GetActorLocation` (`self.As Character`)) (`SceneComponent.K2_GetComponentLocation` (`self.TeleportStartMarker`))) (`KismetMathLibrary.DegAcos` (`KismetMathLibrary.Dot_VectorVector` (`SceneComponent.GetForwardVector` (`self.TeleportStartMarker`)) (`SceneComponent.GetForwardVector` (`self.TeleportTarget`)))) (0.0 0.0 1.0)) (`SceneComponent.K2_GetComponentLocation` (`self.TeleportTarget`))) false false)
        ; Fix the velocity when rotating
        (set `MovementComponent.Velocity` (* (`self.GetVelocity` _as_character) (`KismetMathLibrary.Normal` (`KismetMathLibrary.MakeVector` _returnvalue_roll_3 _returnvalue_pitch_3 _returnvalue_yaw_3))) (`Character.CharacterMovement` _as_character))
        ; Change Rotation
        (`Controller.SetControlRotation` (`Pawn.GetController` _as_character) (`KismetMathLibrary.MakeRotator` _returnvalue_roll_2 _returnvalue_pitch_2 (+ (- _returnvalue_yaw_2 _returnvalue_yaw) _returnvalue_yaw_3)))))
    (:`Is Not Valid`
      (bind _asbp_first_person_character (cast `/Game/FirstPerson/Blueprints/BP_FirstPersonCharacter` OtherActor))
      ;[1 0.25 0 0.5] Replace Cast to Character with Cast to [PLAYER]
      (`KismetSystemLibrary.PrintString` (`KismetSystemLibrary.GetDisplayName` _asbp_first_person_character))
      (set `self.As Character` _asbp_first_person_character)
      (goto _label))))

(fn `UserConstructionScript`)