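; BP_InfiniteHallway builds a seemingly endless corridor along Y, with a door that retreats from the approaching player.
; A box overlap records the starting door distance; Tick then smooths the door away, keeping a gap scaled by SpawnsLeft.
; Every 750 units of door travel spawns another hall light segment and child actor.
; At zero SpawnsLeft, it spawns a corner and moves BP_EndTeleport's start marker; only unconnected logic decrements that counter here.
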(event `self.ReceiveBeginPlay`
  (bind (_returnvalue_x _returnvalue_y _returnvalue_z) (`KismetMathLibrary.BreakVector` (`self.K2_GetActorLocation`)))
  (bind (_returnvalue_x_2 _returnvalue_y_2) (`KismetMathLibrary.BreakVector` (`SceneComponent.K2_GetComponentLocation` (`self.DefaultSceneRoot`))))
  (bind _output_get (set `self.OriginLocation` _returnvalue_y_2))
  (`|SpawnActorFromClass` "/Game/Blueprints/Kitbash/Segments/Hallway/BP_MedHall-Light.BP_MedHall-Light_C" (`KismetMathLibrary.MakeTransform` (`KismetMathLibrary.MakeVector` _returnvalue_x (+ _output_get 750.0) _returnvalue_z) (struct :`Yaw` 90.0)) "Undefined" "MultiplyWithRoot" null null))

(event `self.ReceiveTick`
  (params (DeltaSeconds :type "Float (single-precision)"))
  (bind (_returnvalue_x _returnvalue_y _returnvalue_z) (`KismetMathLibrary.BreakVector` (`self.K2_GetActorLocation`)))
  (bind _movingdoor (`self.MovingDoor`))
  (bind _originlocation (`self.OriginLocation`))
  (bind (_returnvalue_x_2 _returnvalue_y_2) (`KismetMathLibrary.BreakVector` (`self.K2_GetActorLocation` (`self.As BP First Person Character`))))
  (bind (_returnvalue_x_3 _returnvalue_y_3 _returnvalue_z_2) (`KismetMathLibrary.BreakVector` (`SceneComponent.K2_GetComponentLocation` (`self.MovingDoor`))))
  (bind (_returnvalue_x_4 _returnvalue_y_4) (`KismetMathLibrary.BreakVector` (`SceneComponent.K2_GetComponentLocation` _movingdoor)))
  (bind _returnvalue (* (`self.DoorDistance`) (/ (`self.SpawnsLeft`) 3)))
  (if (`self.isMoving`)
    (if (> (`self.SpawnsLeft`) 0)
      (if (<= (- _returnvalue_y_3 _returnvalue_y_2) _returnvalue)
        (`SceneComponent.K2_SetWorldLocation` _movingdoor (`KismetMathLibrary.MakeVector` _returnvalue_x_3 (`KismetMathLibrary.WeightedMovingAverage_Float` (+ _returnvalue _returnvalue_y_2) _returnvalue_y_3 0.1) _returnvalue_z_2) false false)
        (if (and (>= (`KismetMathLibrary.Abs` (- _returnvalue_y_4 _originlocation)) 750.0) (> (`self.SpawnsLeft`) 0))
          (bind _output_get (set `self.OriginLocation` (+ _originlocation 750.0)))
          (bind _returnvalue_2 (+ _output_get 750.0))
          (`|SpawnActorFromClass` "/Game/Blueprints/Kitbash/Segments/Hallway/BP_MedHall-Light.BP_MedHall-Light_C" (`KismetMathLibrary.MakeTransform` (`KismetMathLibrary.MakeVector` _returnvalue_x _returnvalue_2 _returnvalue_z) (struct :`Yaw` 90.0)) "Undefined" "MultiplyWithRoot" null null)
          (bind _returnvalue_3 (`AddComponent|NODE_AddChildActorComponent-2` :`bManualAttachment` true))
          (`SceneComponent.K2_SetWorldLocation` _returnvalue_3 (+ (`KismetMathLibrary.MakeVector` _returnvalue_x _returnvalue_2 _returnvalue_z) (120.0 0.0 100.0)) false false)))
      (else
        (`/Engine/EditorBlueprintResources/StandardMacros.DoOnce` false
          (:`Completed`
            (`self.SpawnEndHallway`)))))))

(event `SpawnEndHallway`
  (bind (_returnvalue_x _returnvalue_y _returnvalue_z) (`KismetMathLibrary.BreakVector` (`self.K2_GetActorLocation`)))
  (bind _originlocation (`self.OriginLocation`))
  (`|SpawnActorFromClass` "/Game/Blueprints/Kitbash/Segments/Hallway/BP_HallCorner.BP_HallCorner_C" (`KismetMathLibrary.MakeTransform` (`KismetMathLibrary.MakeVector` _returnvalue_x (+ _originlocation 1500.0) _returnvalue_z)) "Undefined" "MultiplyWithRoot" null null)
  (bind _returnvalue (`GameplayStatics.GetActorOfClass` "/Game/Blueprints/Tech/BP_EndTeleport.BP_EndTeleport_C"))
  (`SceneComponent.K2_SetWorldLocation` (`/Game/Blueprints/Tech/BP_EndTeleport.TeleportStartMarker` _returnvalue) (`KismetMathLibrary.MakeVector` _returnvalue_x (+ _originlocation 750.0) _returnvalue_z) false false))

(event `self.Box.OnComponentBeginOverlap`
  (params (OverlappedComponent :type "PrimitiveComponent Object Reference") (OtherActor :type "Actor Object Reference") (OtherComp :type "PrimitiveComponent Object Reference") (OtherBodyIndex :type Integer) (bFromSweep :type Boolean) (SweepResult :type "HitResult Structure (by ref)"))
  (bind (_returnvalue_x _returnvalue_y) (`KismetMathLibrary.BreakVector` (`self.K2_GetActorLocation` (`self.As BP First Person Character`))))
  (bind (_returnvalue_x_2 _returnvalue_y_2) (`KismetMathLibrary.BreakVector` (`SceneComponent.K2_GetComponentLocation` (`self.MovingDoor`))))
  (bind _asbp_first_person_character (cast `/Game/FirstPerson/Blueprints/BP_FirstPersonCharacter` OtherActor))
  (set `self.As BP First Person Character` _asbp_first_person_character)
  (`/Engine/EditorBlueprintResources/StandardMacros.DoOnce` false
    (:`Completed`
      (set `self.isMoving` true)
      (set `self.DoorDistance` (- _returnvalue_y_2 _returnvalue_y)))))

(fn `UserConstructionScript`)