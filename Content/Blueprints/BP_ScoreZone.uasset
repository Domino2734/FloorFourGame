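; BP_ScoreZone is a trigger volume that adds or subtracts points from the first-person character's score when it overlaps the Box component.
; On BeginPlay, UpdateScoreValue converts the Score tier, ranging from Big Bad to Big Good, into a negative or positive PointsValue.
; Each qualifying overlap applies that value and prints the new total, with TriggerOnce optionally limiting the zone to a single award via the Triggered flag.
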(event `self.ReceiveBeginPlay`
  (`self.UpdateScoreValue`))

(event `self.ReceiveActorBeginOverlap`
  (params (OtherActor :type "Actor Object Reference")))

(event `self.Box.OnComponentBeginOverlap`
  (params (OverlappedComponent :type "PrimitiveComponent Object Reference") (OtherActor :type "Actor Object Reference") (OtherComp :type "PrimitiveComponent Object Reference") (OtherBodyIndex :type Integer) (bFromSweep :type Boolean) (SweepResult :type "HitResult Structure (by ref)"))
  (bind _asbp_first_person_character (cast `/Game/FirstPerson/Blueprints/BP_FirstPersonCharacter` OtherActor))
  (if (`self.TriggerOnce`)
    (if (not (`self.Triggered`))
      (bind _output_get (set `/Game/FirstPerson/Blueprints/BP_FirstPersonCharacter.Score` (+ (`/Game/FirstPerson/Blueprints/BP_FirstPersonCharacter.Score` _asbp_first_person_character) (`self.PointsValue`)) _asbp_first_person_character :!label _label))
      (set `self.Triggered` true)
      (`KismetSystemLibrary.PrintString` (`KismetStringLibrary.Conv_DoubleToString` _output_get)))
    (else
      (goto _label))))

(fn `UpdateScoreValue`
  (switch `/Game/Blueprints/Enums/EN_ScoreValues` (`self.Score`)
    (:`NewEnumerator0`
      (set `self.PointsValue` -30.0))
    (:`NewEnumerator1`
      (set `self.PointsValue` -15.0))
    (:`NewEnumerator4`
      (set `self.PointsValue` -7.0))
    (:`NewEnumerator5`
      (set `self.PointsValue` 7.0))
    (:`NewEnumerator2`
      (set `self.PointsValue` 15.0))
    (:`NewEnumerator3`
      (set `self.PointsValue` 30.0)))
  (return))

(fn `UserConstructionScript`)