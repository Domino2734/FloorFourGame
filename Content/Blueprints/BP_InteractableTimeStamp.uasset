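; BP_InteractableTimeStamp is an interactable child actor of BP_InfiniteHallway that affects the player's score and the hallway's remaining spawns.
; On BeginPlay it sets its Score enum, runs the parent logic and adds Points to the first-person character's Score.
; The Triggered event runs once, decrementing the parent hallway's SpawnsLeft and subtracting the same Points from the character's Score.
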(event `self.ReceiveBeginPlay`
  (set `self.Score` "NewEnumerator4")
  (`parent.ReceiveBeginPlay`)
  (bind _asbp_first_person_character (cast `/Game/FirstPerson/Blueprints/BP_FirstPersonCharacter` (`GameplayStatics.GetPlayerCharacter` 0)))
  (set `/Game/FirstPerson/Blueprints/BP_FirstPersonCharacter.Score` (+ (`/Game/FirstPerson/Blueprints/BP_FirstPersonCharacter.Score` _asbp_first_person_character) (`self.Points`)) _asbp_first_person_character))

(event `self.Triggered`
  (`/Engine/EditorBlueprintResources/StandardMacros.DoOnce` false
    (:`Completed`
      (bind _asbp_infinite_hallway (cast `/Game/Blueprints/Tech/BP_InfiniteHallway` (`self.GetParentActor`)))
      (`/Engine/EditorBlueprintResources/StandardMacros.DecrementInt` (`/Game/Blueprints/Tech/BP_InfiniteHallway.SpawnsLeft` _asbp_infinite_hallway)
        (:`  `
          (bind _asbp_first_person_character (cast `/Game/FirstPerson/Blueprints/BP_FirstPersonCharacter` (`GameplayStatics.GetPlayerCharacter` 0)))
          (set `/Game/FirstPerson/Blueprints/BP_FirstPersonCharacter.Score` (+ (`/Game/FirstPerson/Blueprints/BP_FirstPersonCharacter.Score` _asbp_first_person_character) (* (`self.Points`) -1.0)) _asbp_first_person_character))))))

(fn `UserConstructionScript`
  (`parent.UserConstructionScript`))