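; Interactable door Blueprint with a trigger event and basic open and lock state.
; Triggered snaps the static mesh to a fixed relative rotation, without checking IsLocked or setting IsOpen.
; CloseDoor only clears IsOpen and does not rotate the mesh back; LockDoor calls it, then sets IsLocked.
; Tick is empty, and a leftover local-rotation node is never executed.
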(event `self.ReceiveTick`
  (params (DeltaSeconds :type "Float (single-precision)")))

(event `self.Triggered`
  (`SceneComponent.K2_SetRelativeRotation` (`self.StaticMesh`) (struct :`Yaw` 90.0) false false))

(event `CloseDoor`
  (if (`self.isOpen`)
    (set `self.isOpen` false)))

(event `LockDoor`
  (`self.CloseDoor`)
  (set `self.isLocked` true))

(fn `UserConstructionScript`
  (`parent.UserConstructionScript`))